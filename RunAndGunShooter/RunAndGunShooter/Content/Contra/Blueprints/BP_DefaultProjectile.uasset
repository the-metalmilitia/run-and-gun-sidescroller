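; BP_DefaultProjectile is a pooled projectile that returns itself to its owning pool on timeout or overlap.
; While active, Tick accumulates activation time and triggers the return once the auto-deactivation timer is reached.
; A CollisionSphere begin-overlap triggers the same return without filtering the other actor.
; Both paths then share one debug print chain, so the hit messages also print on timeout.
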(event OnComponentBeginOverlap(CollisionSphere)
  (params (OverlappedComponent :type Primitive%20Component%20Object%20Reference) (OtherActor :type Actor%20Object%20Reference) (OtherComp :type Primitive%20Component%20Object%20Reference) (OtherBodyIndex :type Integer) (bFromSweep :type Boolean) (SweepResult :type Hit%20Result%20Structure%20%28by%20ref%29))
  (bind _self self)
  (Class|ProjectileDataManager|ReturnProjectiletoPool (Class|ProjectileBase|GetOwningPool _self) _self)
  (Development|PrintText (Utilities|Text|ToText(Object) _self))
  (Development|PrintText "Took the projectile")
  (Development|PrintString (Utilities|GetObjectName OtherActor))
  (Development|PrintText "Got hit"))

(event EventBeginPlay)

(event Collision|EventActorBeginOverlap
  (params (OtherActor :type Actor%20Object%20Reference)))

(event EventTick
  (params (DeltaSeconds :type Float%20%28single-precision%29))
  (bind _self self)
  (if (Class|ProjectileBase|IsProjectileActive self)
    (bind _output_get (Variables|Default|SetCurrentActivationTime (+ DeltaSeconds (Variables|Default|GetCurrentActivationTime))))
    (if (>= _output_get (Variables|Default|GetAutoDeactivationTimer))
      (Class|ProjectileDataManager|ReturnProjectiletoPool (Class|ProjectileBase|GetOwningPool _self) _self)
      (Development|PrintText (Utilities|Text|ToText(Object) self))
      (Development|PrintText "Took the projectile")
      (Development|PrintString (Utilities|GetObjectName (stale OnComponentBeginOverlap(CollisionSphere) OtherActor)))
      (Development|PrintText "Got hit"))))

(fn ConstructionScript)